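; BP_HealthPack is a short-lived health pickup that heals the player on touch and expires ten seconds after spawning.
; Its static mesh overlap casts the other actor to BP_Player, adds a fixed amount of health capped at full, and updates the player's health bar widget.
; The pack then destroys itself, while non-player overlaps are ignored.
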(event `self.ReceiveBeginPlay`
  (`self.SetLifeSpan` 10.0))

(event `self.StaticMesh.OnComponentBeginOverlap`
  (params (OverlappedComponent :type "PrimitiveComponent Object Reference") (OtherActor :type "Actor Object Reference") (OtherComp :type "PrimitiveComponent Object Reference") (OtherBodyIndex :type Integer) (bFromSweep :type Boolean) (SweepResult :type "HitResult Structure (by ref)"))
  (bind _asbp_player (cast `/Game/InfiniteMatrix/Blueprints/BP_Player` OtherActor))
  (bind _health (`/Game/InfiniteMatrix/Blueprints/BP_Player.Health` _asbp_player))
  (if (<= _health 80.0)
    (set `/Game/InfiniteMatrix/Blueprints/BP_Player.Health` (+ _health 20.0) _asbp_player)
    (else
      (set `/Game/InfiniteMatrix/Blueprints/BP_Player.Health` 100.0 _asbp_player)))
  (`/Game/InfiniteMatrix/Blueprints/WB_HealthBar.UpdateHealthBar` (`/Game/InfiniteMatrix/Blueprints/BP_Player.WB_Healthbar` _asbp_player) (`/Game/InfiniteMatrix/Blueprints/BP_Player.Health` _asbp_player))
  (`self.K2_DestroyActor`))

(fn `UserConstructionScript`)